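; BP_TraceCannon is an actor that appears to be a test bed for collision trace nodes.
; On BeginPlay it runs one multi sphere trace on the Visibility channel forward from its Scene component, with persistent debug drawing.
; It loops over the hits but does nothing with them.
; Unconnected line, box, sphere, capsule, object and multi-line trace nodes remain in the graph and never run.
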(event `self.ReceiveBeginPlay`
  (bind _scene (`self.Scene`))
  (bind _returnvalue (`SceneComponent.K2_GetComponentLocation` _scene))
  (bind _outhits (`KismetSystemLibrary.SphereTraceMulti` :`Start` _returnvalue :`End` (+ _returnvalue (* (`SceneComponent.GetForwardVector` _scene) 1000.0)) :`Radius` 50.0 :`TraceChannel` "TraceTypeQuery1" :`DrawDebugType` "Persistent"))
  (for _array_element _outhits
    _))

(fn `UserConstructionScript`)