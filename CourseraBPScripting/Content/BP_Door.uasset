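; BP_Door is an automatic sliding door that opens when the first player character overlaps it and closes when that overlap ends.
; OpenDoor plays the DoorOpening timeline and CloseDoor reverses it, with the timeline's Position output scaling a sideways Y offset for the Cube's relative location.
; LockDoor and UnlockDoor are empty functions, so the door has no locking behavior.
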(event `self.ReceiveActorBeginOverlap`
  (params (OtherActor :type "Actor Object Reference"))
  (if (== OtherActor (`GameplayStatics.GetPlayerCharacter` 0))
    (`self.OpenDoor`)))

(event `self.ReceiveActorEndOverlap`
  (params (OtherActor :type "Actor Object Reference"))
  (if (== OtherActor (`GameplayStatics.GetPlayerCharacter` 0))
    (`self.CloseDoor`)))

(event `OpenDoor`
  (bind (_direction _position) (`Timeline|DoorOpening` :!label _label)
    (:`Update`
      (`SceneComponent.K2_SetRelativeLocation` (`self.Cube`) (* (0.0 300.0 0.0) _position) false false))))

(event `CloseDoor`
  (goto _label :!via `Reverse`))

(fn `LockDoor`)

(fn `UnlockDoor`)

(fn `UserConstructionScript`)