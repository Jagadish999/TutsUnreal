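; BP_Button is an overlap-activated button that reports when the player character steps on or off it.
; Begin and end overlaps filter for player character 0, then route through ButtonTriggered and ButtonUntriggered events.
; These events broadcast the OnButtonTriggered dispatcher with true or false, leaving any response to bound listeners.
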(event `self.ReceiveActorBeginOverlap`
  (params (OtherActor :type "Actor Object Reference"))
  (if (== OtherActor (`GameplayStatics.GetPlayerCharacter` 0))
    (`self.ButtonTriggered`)))

(event `self.ReceiveActorEndOverlap`
  (params (OtherActor :type "Actor Object Reference"))
  (if (== OtherActor (`GameplayStatics.GetPlayerCharacter` 0))
    (`self.ButtonUntriggered`)))

(event `ButtonTriggered`
  (`self.OnButtonTriggered` true))

(event `ButtonUntriggered`
  (`self.OnButtonTriggered` false))

(fn `UserConstructionScript`)