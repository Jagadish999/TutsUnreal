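; BP_WallButton is an interactable wall button that signals a triggered state for a timed period when pushed.
; Interacting calls OnTriggered with true, moves the cube inward and starts a timer whose length comes from the Timer variable.
; OnButtonTriggered, the apparent timer callback, resets the cube and calls OnTriggered with false.
; LookAt supplies the "Push Button" verb and noun for the interaction.
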(event `/Game/BPI_Interact.InteractWith`
  (params (PlayerCharacter :type "/Game/ThirdPerson/Blueprints/BP_ThirdPersonCharacter Object Reference"))
  (`self.OnTriggered` true)
  (`SceneComponent.K2_SetRelativeLocation` (`self.Cube`) (-10.0 0.0 0.0) false false)
  (`KismetSystemLibrary.K2_SetTimerDelegate` (`|CreateDelegate` :!event `OnButtonTriggered`) (`self.timer`)))

(fn `LookAt`
  (returns (Verb :type String) (Noun :type String))
  (return "Push" "Button"))

(fn `OnButtonTriggered`
  (`SceneComponent.K2_SetRelativeLocation` (`self.Cube`) (0.0 0.0 0.0) false false)
  (`self.OnTriggered` false))

(fn `UserConstructionScript`
  (`parent.UserConstructionScript`))